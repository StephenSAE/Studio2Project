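; Squirrel NPC character that idles, wanders and flees from pawns tagged as player or predator.
; Tick runs randomly delayed loops for idle montages and short navmesh wanders, including a slower loop that moves even if already moving.
; A delayed forward box trace and a per-tick surrounding box trace trigger a faster run to a random, farther navmesh point.
; A DoOnce gates the surrounding trigger, and fleeing repeats until the threat leaves sight.
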(event `self.ReceiveBeginPlay`
  ;[1 1 1] Begin Play
)

(event `Random Animation`
  ;[0.6759 1 0.7569] Random Animation
  (if (not (`self.isMoving`))
    (`self.PlayAnimMontage` (`KismetArrayLibrary.Array_Get` (`self.Squirrel_Montages`) (`KismetMathLibrary.RandomIntegerInRange` 0 1)))
    (else
      (`self.StopAnimMontage` null))))

(event `self.ReceiveTick`
  (params (DeltaSeconds :type "Float (single-precision)"))
  (bind _charactermovement (`self.CharacterMovement`))
  (bind _charactermovement_2 (`self.CharacterMovement`))
  (bind _sightcenter (`self.SightCenter`))
  (bind _front_sensor (`self.Front_Sensor`))
  (bind _returnvalue (`SceneComponent.K2_GetComponentLocation` _front_sensor))
  (bind _returnvalue_2 (`SceneComponent.K2_GetComponentLocation` _sightcenter))
  ;[1 1 1] Event Tick
  (`|ExecutionSequence`
    (:`then_0`
      ;[1 0.575 0.575] Run Random Animation
      (`KismetSystemLibrary.Delay` (`KismetMathLibrary.RandomFloatInRange` 2.0 8.0))
      (`self.Random Animation`))
    (:`then_1`
      ;[1 1 1] Run around
      (`KismetSystemLibrary.Delay` (`KismetMathLibrary.RandomFloatInRange` 5.0 20.0))
      (if (not (`self.isMoving`))
        (`self.StopAnimMontage` null)
        (set `CharacterMovementComponent.MaxWalkSpeed` (`KismetMathLibrary.RandomFloatInRange` 200.0 250.0) _charactermovement_2)
        (set `CharacterMovementComponent.RotationRate` (struct :`Yaw` 200.0) _charactermovement_2)
        (`|AIMoveTo` self (`NavigationSystem.GetRandomPointInNavigableRadius` (`self.K2_GetActorLocation`) 1000.0) null 5.0
          (:`then`
            (set `self.isMoving` true))
          (:`OnSuccess`
            (set `self.isMoving` false)))))
    (:`then_2`
      ;[1 1 1] Run around 2
      (`KismetSystemLibrary.Delay` (`KismetMathLibrary.RandomFloatInRange` 20.0 30.0))
      (`self.StopAnimMontage` null)
      (set `CharacterMovementComponent.MaxWalkSpeed` (`KismetMathLibrary.RandomFloatInRange` 200.0 250.0) _charactermovement)
      (set `CharacterMovementComponent.RotationRate` (struct :`Yaw` 200.0) _charactermovement)
      (`|AIMoveTo` self (`NavigationSystem.GetRandomPointInNavigableRadius` (`self.K2_GetActorLocation`) 1000.0) null 5.0
        (:`then`
          (set `self.isMoving` true))
        (:`OnSuccess`
          (set `self.isMoving` false))))
    (:`then_3`
      ;[1 1 1] Front Sensor
      (`KismetSystemLibrary.Delay` 0.5)
      (bind (_outhit _returnvalue_3) (`KismetSystemLibrary.BoxTraceSingleForObjects` _returnvalue (+ _returnvalue (* (`SceneComponent.GetForwardVector` _front_sensor) 1500.0)) (0.0 150.0 50.0) (`SceneComponent.K2_GetComponentRotation` _front_sensor) (`|MakeArray` "ObjectTypeQuery3" :!type "EObjectTypeQuery Enum")))
      (if _returnvalue_3
        (`|ExecutionSequence`
          (:`then_0`
            (bind (_bblockinghit _binitialoverlap _time _location _impactpoint _normal _impactnormal _physmat _hitactor) (`GameplayStatics.BreakHitResult` _outhit))
            (if (or (`self.ActorHasTag` _hitactor "player") (or (`self.ActorHasTag` _hitactor "predator") (`self.ActorHasTag` _hitactor "predator_2")))
              (`self.Run_Away_Event`))))))
    (:`then_4`
      ;[1 0.8849 0.3424] Run Away
      (bind (_outhit_2 _returnvalue_4) (`KismetSystemLibrary.BoxTraceSingleForObjects` _returnvalue_2 _returnvalue_2 (1000.0 700.0 150.0) (`SceneComponent.K2_GetComponentRotation` _sightcenter) (`|MakeArray` "ObjectTypeQuery3" :!type "EObjectTypeQuery Enum")))
      (if _returnvalue_4
        (bind (_bblockinghit_2 _binitialoverlap_2 _time_2 _location_2 _impactpoint_2 _normal_2 _impactnormal_2 _physmat_2 _hitactor_2) (`GameplayStatics.BreakHitResult` _outhit_2))
        (if (or (`self.ActorHasTag` _hitactor_2 "player") (or (`self.ActorHasTag` _hitactor_2 "predator") (`self.ActorHasTag` _hitactor_2 "predator_2")))
          (set `self.InSight` true)
          (`/Engine/EditorBlueprintResources/StandardMacros.DoOnce` false :!label _label
            (:`Completed`
              (`self.Run_Away_Event`)))
          (else
            (set `self.InSight` false :!label _label_2)))
        (else
          (goto _label_2))))))

(event `Run_Away_Event`
  (bind _charactermovement (`self.CharacterMovement`))
  ;[1 1 1] Run Away Event
  (`self.StopAnimMontage` null)
  (set `CharacterMovementComponent.MaxWalkSpeed` 500.0 _charactermovement)
  (set `CharacterMovementComponent.RotationRate` (struct :`Yaw` 400.0) _charactermovement)
  (`|AIMoveTo` self (`NavigationSystem.GetRandomPointInNavigableRadius` (`self.K2_GetActorLocation`) (`KismetMathLibrary.RandomFloatInRange` 1750.0 5000.0)) null 15.0
    (:`then`
      (set `self.isMoving` true))
    (:`OnSuccess`
      (set `self.isMoving` false)
      (if (`self.InSight`)
        (`self.Run_Away_Event`)
        (else
          (goto _label :!via `Reset`))))))

(fn `UserConstructionScript`)
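; BP_WidgetTest1 is a test actor that shows and hides a WBP_TestWidge1 screen widget through a trigger volume.
; Begin overlap creates and caches the widget if missing, or adds the cached one to the viewport; the creation branch does not display it.
; End overlap removes the widget, but PlayerInRange is never cleared.
; Overlaps are not filtered by actor, and the Player_Character casts lead to no action.
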(event `self.TriggerVolume.OnComponentBeginOverlap`
  (params (OverlappedComponent :type "PrimitiveComponent Object Reference") (OtherActor :type "Actor Object Reference") (OtherComp :type "PrimitiveComponent Object Reference") (OtherBodyIndex :type Integer) (bFromSweep :type Boolean) (SweepResult :type "HitResult Structure (by ref)"))
  (set `self.PlayerInRange` true)
  (if (`self.WidgetActive`)
    _
    (elif (`KismetSystemLibrary.IsValid` (`self.WidgetDisplay1`))
      (`self.AddWidget`)
      (else
        (bind _returnvalue (`|CreateWidget` "/Game/_Widgets/WBP_TestWidge1.WBP_TestWidge1_C" (`GameplayStatics.GetPlayerController` 0)))
        (set `self.WidgetDisplay1` _returnvalue)))))

(event `self.TriggerVolume.OnComponentEndOverlap`
  (params (OverlappedComponent :type "PrimitiveComponent Object Reference") (OtherActor :type "Actor Object Reference") (OtherComp :type "PrimitiveComponent Object Reference") (OtherBodyIndex :type Integer))
  (`self.RemoveWidget`))

(event `AddWidget`
  (`UserWidget.AddToViewport` (`self.WidgetDisplay1`) 0)
  (set `self.WidgetActive` true)
  (cast `/Game/_BluePrints/Player_Character/Player_Character` (`GameplayStatics.GetPlayerCharacter` 0)))

(event `RemoveWidget`
  (`Widget.RemoveFromParent` (`self.WidgetDisplay1`))
  (set `self.WidgetActive` false)
  (cast `/Game/_BluePrints/Player_Character/Player_Character` (`GameplayStatics.GetPlayerCharacter` 0)))

(fn `UserConstructionScript`)
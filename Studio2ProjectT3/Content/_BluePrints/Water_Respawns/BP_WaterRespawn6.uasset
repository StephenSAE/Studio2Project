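; BP_WaterRespawn6 is a water respawn trigger that returns the player to a fixed location.
; Any overlap with its Box creates a WBP_TeleporterFade widget, waits out a short delay, teleports player character 0 to hardcoded coordinates, then removes the widget.
; The overlapping actor is not checked.
; A StartFade event and a disconnected validity check remain from an earlier attempt and are unused.
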(event `self.Box.OnComponentBeginOverlap`
  (params (OverlappedComponent :type "PrimitiveComponent Object Reference") (OtherActor :type "Actor Object Reference") (OtherComp :type "PrimitiveComponent Object Reference") (OtherBodyIndex :type Integer) (bFromSweep :type Boolean) (SweepResult :type "HitResult Structure (by ref)"))
  (bind _returnvalue (`|CreateWidget` "/Game/_Widgets/WBP_TeleporterFade.WBP_TeleporterFade_C" (`GameplayStatics.GetPlayerController` 0)))
  (set `self.TeleportFadeWidge` _returnvalue)
  (`UserWidget.AddToViewport` (`self.TeleportFadeWidge`) 0)
  (`KismetSystemLibrary.Delay` 2.5)
  (`self.K2_TeleportTo` (`GameplayStatics.GetPlayerCharacter` 0) (8670.0 7540.0 300.0) (struct :`Yaw` -140.0))
  (`Widget.RemoveFromParent` (`self.TeleportFadeWidge`)))

(event `Start Fade`
  ;[1 0 0.007345] Attempt1
  (`UserWidget.AddToViewport` (`self.TeleportFadeWidge`) 0))

(fn `UserConstructionScript`)
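; BP_WaterRespawn9 is a water respawn trigger that returns the player to a hardcoded location.
; Any overlap on its Box creates a WBP_TeleporterFade widget, calls Respawning on player 0's Player_Character and shows the fade, without checking the overlapping actor.
; After a delay it teleports the character, clears its Shot flag and removes the widget.
; StartFade and two disconnected chains remain from earlier attempts.
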(event `self.Box.OnComponentBeginOverlap`
  (params (OverlappedComponent :type "PrimitiveComponent Object Reference") (OtherActor :type "Actor Object Reference") (OtherComp :type "PrimitiveComponent Object Reference") (OtherBodyIndex :type Integer) (bFromSweep :type Boolean) (SweepResult :type "HitResult Structure (by ref)"))
  (bind _returnvalue (`GameplayStatics.GetPlayerCharacter` 0))
  (bind _returnvalue_2 (`|CreateWidget` "/Game/_Widgets/WBP_TeleporterFade.WBP_TeleporterFade_C" (`GameplayStatics.GetPlayerController` 0)))
  (set `self.TeleportFadeWidge` _returnvalue_2)
  (bind _asplayer_character (cast `/Game/_BluePrints/Player_Character/Player_Character` _returnvalue)
    (:`then`
      (`/Game/_BluePrints/Player_Character/Player_Character.Respawning` _asplayer_character)
      (`UserWidget.AddToViewport` (`self.TeleportFadeWidge`) 0)
      (`KismetSystemLibrary.Delay` 2.5)
      (`self.K2_TeleportTo` _returnvalue (2050.0 8980.0 460.0) (struct :`Yaw` -140.0))
      (bind _asplayer_character_2 (cast `/Game/_BluePrints/Player_Character/Player_Character` _returnvalue)
        (:`then`
          (set `/Game/_BluePrints/Player_Character/Player_Character.Shot` false _asplayer_character_2)
          (`Widget.RemoveFromParent` (`self.TeleportFadeWidge`)))
        (:`CastFailed`
          (`KismetSystemLibrary.PrintString` "Player not found OwO"))))
    (:`CastFailed`
      (`KismetSystemLibrary.PrintString` "Player not found OwO"))))

(event `Start Fade`
  ;[1 0 0.007345] Attempt1
  (`UserWidget.AddToViewport` (`self.TeleportFadeWidge`) 0))

(fn `UserConstructionScript`)
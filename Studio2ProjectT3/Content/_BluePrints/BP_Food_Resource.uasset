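; BP_Food_Resource is a food source that visually depletes as its Food value drops.
; BeginPlay fills Food from StartingFood, and Tick is unused.
; UpdateFood hides three passed-in food groups in stages: below full, at half or less, and at empty, when it also deactivates the particle effect.
; It only hides, never re-shows or destroys, and this graph neither reduces Food nor calls UpdateFood.
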(event `self.ReceiveBeginPlay`
  (set `self.Food` (`self.Starting Food`)))

(fn `Update Food`
  (params (`Food Group 1` :type "SceneComponent Object Reference") (`Food Group 2` :type "SceneComponent Object Reference") (`Food Group 3` :type "SceneComponent Object Reference") (`Particle Effect` :type "ParticleSystemComponent Object Reference"))
  (bind _food (`self.Food`))
  (bind _starting_food (`self.Starting Food`))
  (if (< _food _starting_food)
    ;[1 1 1] Hide First Food Group
    (`SceneComponent.SetVisibility` `Food Group 1` false true)
    (if (<= _food (/ _starting_food 2.0))
      ;[1 1 1] Hide Second Food Group
      (`SceneComponent.SetVisibility` `Food Group 2` false true)
      (if (<= _food 0.0)
        ;[1 1 1] Destroy all food groups and particle Effect
        (`SceneComponent.SetVisibility` `Food Group 3` false true)
        (`self.SetActive` `Particle Effect` false false)))))
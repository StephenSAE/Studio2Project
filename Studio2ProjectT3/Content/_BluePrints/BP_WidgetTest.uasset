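; BP_WidgetTest is a test Blueprint that toggles a WBP_TestWidge screen widget through a trigger volume.
; Begin overlap adds the cached widget to the viewport, or only creates it if none exists, so the first overlap displays nothing.
; End overlap removes it, with WidgetActive guarding against repeat adds.
; Overlaps are not filtered by actor, and PlayerInRange is set but never cleared by live logic.
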(event `self.TriggerVolume.OnComponentBeginOverlap`
  (params (OverlappedComponent :type "PrimitiveComponent Object Reference") (OtherActor :type "Actor Object Reference") (OtherComp :type "PrimitiveComponent Object Reference") (OtherBodyIndex :type Integer) (bFromSweep :type Boolean) (SweepResult :type "HitResult Structure (by ref)"))
  (set `self.PlayerInRange` true)
  (if (`self.WidgetActive`)
    _
    (elif (`KismetSystemLibrary.IsValid` (`self.WidgetDisplay`))
      (`self.AddWidget`)
      (else
        (bind _returnvalue (`|CreateWidget` "/Game/_Widgets/WBP_TestWidge.WBP_TestWidge_C" (`GameplayStatics.GetPlayerController` 0)))
        (set `self.WidgetDisplay` _returnvalue)))))

(event `self.TriggerVolume.OnComponentEndOverlap`
  (params (OverlappedComponent :type "PrimitiveComponent Object Reference") (OtherActor :type "Actor Object Reference") (OtherComp :type "PrimitiveComponent Object Reference") (OtherBodyIndex :type Integer))
  (`self.RemoveWidget`))

(event `AddWidget`
  (`UserWidget.AddToViewport` (`self.WidgetDisplay`) 0)
  (set `self.WidgetActive` true))

(event `RemoveWidget`
  (`Widget.RemoveFromParent` (`self.WidgetDisplay`))
  (set `self.WidgetActive` false))

(fn `UserConstructionScript`)